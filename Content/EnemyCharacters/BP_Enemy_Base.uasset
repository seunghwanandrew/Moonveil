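; Base enemy Blueprint that handles the death sequence by dissolving the enemy and its equipped weapon.
; On death it pauses mesh animation, disables capsule collision and async-loads a Niagara effect attached to the mesh.
; The particle color is copied from the mesh material's dissolve edge color.
; A timeline scaled to the total dissolve time drives DissolveAmount on both meshes, then destroys weapon and actor.
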(event EventBeginPlay)

(event Collision|EventActorBeginOverlap
  (params (OtherActor :type Actor%20Object%20Reference)))

(event EventTick
  (params (DeltaSeconds :type Float%20%28single-precision%29)))

(event EventOnEnemyDied
  (params (DissoloveNiagaraSystem :type Niagara%20System%20Soft%20Object%20Reference))
  (bind _mesh (Variables|Character|GetMesh))
  (bind _enemycombatcomponent (Variables|Default|GetEnemyCombatComponent))
  (bind _enemycombatcomponent_2 (Variables|Default|GetEnemyCombatComponent))
  (bind _returnvalue (Class|MoonveilBaseCombatComponent|GetCharacterCurrentEquippedWeapon _enemycombatcomponent))
  (bind _returnvalue_2 (Class|MoonveilBaseCombatComponent|GetCharacterCurrentEquippedWeapon _enemycombatcomponent_2))
  (bind _weaponmesh (Variables|/Script/Moonveil.MoonveilBaseWeapon|GetWeaponMesh _returnvalue_2))
  (Variables|Default|SetDissolove%20Niagara%20System DissoloveNiagaraSystem)
  (Utilities|FlowControl|Sequence
    (:then_0
      ;[0.15 0.15 0.15 0.5] Disable Collision and Anim
      (Variables|/Script/Engine.SkeletalMeshComponent|SetbPauseAnims (Variables|Character|GetMesh) true)
      (Collision|SetCollisionEnabled (Variables|Default|GetCapsuleComponent) "NoCollision"))
    (:then_1
      ;[0.15 0.15 0.15 0.5] Spawn Niagaram System Effect
      (bind _object (Utilities|AsyncLoadAsset (Variables|Default|GetDissolove%20Niagara%20System))
        (:Completed
          (bind _asniagara_system (Utilities|Casting|CastToNiagaraSystem _object))
          (bind _returnvalue_3 (Niagara|SpawnSystemAttached _asniagara_system (Variables|Character|GetMesh) "None" "0, 0, 0" "0, 0, 0" "KeepRelativeOffset" false))
          (bind _returnvalue_4 (Rendering|Material|CreateDynamicMaterialInstance _mesh 0 (Rendering|Material|GetMaterial _mesh 0) "None" :!class /Script/Engine.PrimitiveComponent))
          (bind _returnvalue_5 (Rendering|Material|GetVectorParameterValue _returnvalue_4 "DissolveEdgeColor" :!class /Script/Engine.MaterialInstanceDynamic))
          (Niagara|SetNiagaraVariable(LinearColor) _returnvalue_3 "DissolveParticleColor" _returnvalue_5))))
    (:then_2
      ;[0.15 0.15 0.15 0.5] Dissolve Enemy And Weapon
      (Components|Timeline|SetPlayRate (Variables|Default|GetDissolve%20Timeline) (/ 1.0 (Variables|Default|GetTotal%20Dissolve%20Time)))
      (bind _normalized_float_track (Timeline|Dissolve%20Timeline PlayFromStart)
        (:Update
          (Utilities|FlowControl|Sequence
            (:then_0
              (Utilities|IsValid _weaponmesh
                (:Is%20Valid
                  (Rendering|Material|SetScalarParameterValueonMaterials _weaponmesh "DissolveAmount" _normalized_float_track))))
            (:then_1
              (Rendering|Material|SetScalarParameterValueonMaterials (Variables|Character|GetMesh) "DissolveAmount" _normalized_float_track))))
        (:Finished
          ;[0.15 0.15 0.15 0.5] Destroy Weapon & Self Actor
          (Utilities|IsValid _returnvalue
            (:Is%20Valid
              (Actor|DestroyActor _returnvalue))
            (:Is%20Not%20Valid
              _))
          (Actor|DestroyActor))))))

(fn ConstructionScript)